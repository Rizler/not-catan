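; BP_Tile is a board tile for NotCatan whose look reflects its tile type and resource.
; The UpdateMaterial event hides the static mesh for NONE tiles and sets the decal material for RESOURCE tiles by switching on the resource, from desert to lumber.
; A sea material assignment exists but is unconnected, and the construction script and other events are empty.
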(event EventBeginPlay)

(event Collision|EventActorBeginOverlap
  (params (OtherActor :type Actor%20Object%20Reference)))

(event EventTick
  (params (DeltaSeconds :type Float%20%28single-precision%29)))

(event EventUpdateMaterial
  (switch Utilities|FlowControl|Switch|SwitchonETileType (Variables|Default|Getm_tileType)
    (:NONE
      (Rendering|SetVisibility (Variables|Default|GetStaticMesh) false false))
    (:RESOURCE
      (switch Utilities|FlowControl|Switch|SwitchonEResource (Variables|Default|Getm_resource)
        (:DESERT
          (Variables|Default|SetNew%20Material "/Game/NotCatan/Materials/M_Desert.M_Desert"))
        (:GRAIN
          (Variables|Default|SetNew%20Material "/Game/NotCatan/Materials/M_Grain.M_Grain"))
        (:WOOL
          (Variables|Default|SetNew%20Material "/Game/NotCatan/Materials/M_Wool.M_Wool"))
        (:BRICK
          (Variables|Default|SetNew%20Material "/Game/NotCatan/Materials/M_Brick.M_Brick"))
        (:ORE
          (Variables|Default|SetNew%20Material "/Game/NotCatan/Materials/M_Ore.M_Ore"))
        (:LUMBER
          (Variables|Default|SetNew%20Material "/Game/NotCatan/Materials/M_Lumber.M_Lumber")))
      (Rendering|Components|Decal|SetDecalMaterial (Variables|Default|GetDecal) (Variables|Default|GetNew%20Material)))))

(fn ConstructionScript)